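; BP_BurningBush is a bush actor that catches fire, spreads it to overlapping bushes and burns away.
; FireSpread steps the particle effect from small to large fire on delays, then calls FireSpread on overlapping bushes tagged "Burn".
; It removes each neighbor's tag first, preventing repeat ignition from spreading.
; Burnout sits inside that loop, so hiding the fire, applying the burnt material and destroying the actor require a tagged neighbor.
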(event `Fire Spread`
  (bind _particlesystem (`self.ParticleSystem`))
  (`ParticleSystemComponent.SetTemplate` _particlesystem "/Game/Particles/Small_Fire.Small_Fire")
  (`KismetSystemLibrary.Delay` 5.0)
  (`ParticleSystemComponent.SetTemplate` _particlesystem "/Game/Particles/Large_Fire.Large_Fire")
  (`KismetSystemLibrary.Delay` 5.0)
  (for _array_element (`self.GetOverlappingActors` "BP_BurningBush_C")
    (if (`self.ActorHasTag` _array_element "Burn")
      (`KismetArrayLibrary.Array_RemoveItem` (`Actor.Tags` _array_element) "Burn")
      (bind _asbp_burning_bush (cast `/Game/Blueprint/BP_BurningBush` _array_element))
      (`self.Fire Spread` _asbp_burning_bush)
      (`KismetSystemLibrary.Delay` 2.0)
      (`SceneComponent.SetHiddenInGame` (`self.ParticleSystem`) true true)
      (`PrimitiveComponent.SetMaterial` (`self.StaticMesh`) 0 "/Game/Materials/Burnt_Bush_Mat.Burnt_Bush_Mat")
      (`KismetSystemLibrary.Delay` 10.0)
      (`self.K2_DestroyActor`))))

(fn `UserConstructionScript`)